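; Door actor that the player opens and closes with the F key while near it.
; Overlap with the Box component enables input for player controller 0 and end overlap disables it, without checking which actor overlaps.
; F flips the DoorStatus flag and alternately plays or reverses the OpenCloseDoor timeline.
; The timeline's DoorRotation track sets the whole actor's absolute yaw, with pitch and roll at zero.
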(event OnComponentBeginOverlap(Box)
  (params (OtherActor :type Actor%20Object%20Reference) (OtherComp :type Primitive%20Component%20Object%20Reference) (OtherBodyIndex :type Integer) (bFromSweep :type Boolean) (SweepResult :type Hit%20Result%20Structure%20%28by%20ref%29))
  ;[1 1 1] Permite que puedas abrir la puerta
  (Input|EnableInput (Game|GetPlayerController 0)))

(event OnComponentEndOverlap(Box)
  (params (OtherActor :type Actor%20Object%20Reference) (OtherComp :type Primitive%20Component%20Object%20Reference) (OtherBodyIndex :type Integer))
  ;[1 1 1] Permite que puedas abrir la puerta
  (Input|DisableInput (Game|GetPlayerController 0)))

(event Input|KeyboardEvents|F
  (params (Key :type Key%20Structure :default "AnyKey"))
  ;[1 1 1] Abrir/Cerrar Puerta
  (:Pressed
    (if (Variables|Default|GetDoorStatus)
      (Variables|Default|SetDoorStatus false)
      (bind _doorrotation (Timeline|OpenCloseDoor Play)
        (:Update
          (Transformation|SetActorRotation (Math|Rotator|MakeRotator 0.0 0.0 _doorrotation))))
      (else
        (Variables|Default|SetDoorStatus true)
        (Timeline|OpenCloseDoor Reverse)))))

(fn ConstructionScript)